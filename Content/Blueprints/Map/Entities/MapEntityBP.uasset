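; Blueprint for a map entity, friendly or enemy, that handles its visual and audio feedback on a cell-based map.
; Movement, attack and damage events trigger Niagara effects and sounds, and non-friendly entities get a teleport effect shortly after spawning.
; A billboard shows a selection icon by allegiance and attack state, while a shield appears whenever health is above one.
; Death destroys the actor.
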(event `self.ReceiveBeginPlay`
  (`|ExecutionSequence`
    (:`then_0`
      (`SceneComponent.SetVisibility` (`self.Billboard`) false false)
      (`self.UpdateShield`)
      (add `self.OnMove` (`|CreateDelegate` :!event `MoveEvent`))
      (add `self.OnAttack` (delegate `Attack`)))
    (:`then_1`
      (`KismetSystemLibrary.Delay` 0.01)
      (if (not (`self.GetIsFriendly`))
        (`NiagaraFunctionLibrary.SpawnSystemAtLocation` "/Game/VFX/Spawn/VFX_SpawnEnemy.VFX_SpawnEnemy" (`self.K2_GetActorLocation`))
        (`GameplayStatics.PlaySound2D` "/Game/SFX/Teleport.Teleport" 0.2 1.0 0.0 null null)))))

(event `Attack` :!signature `self.OnAttack`
  (params (MapEntity :type "MapEntity Object Reference") (AttackInfo :type "MapAttackInfo Structure (by ref)"))
  (`GameplayStatics.PlaySound2D` "/Game/SFX/Attack.Attack" 1.0 1.0 0.0 null null))

(event `MoveEvent` :!signature `self.OnMove`
  (params (MapEntity :type "MapEntity Object Reference") (FromCell :type "HexCell Object Reference") (ToCell :type "HexCell Object Reference"))
  (bind _returnvalue (select `bool` (`self.GetIsFriendly`) :`false` "/Game/VFX/Move/VFX_MoveEnemy.VFX_MoveEnemy" :`true` "/Game/VFX/Move/VFX_MovePlayer.VFX_MovePlayer" :!type "NiagaraSystem Object Reference"))
  (`/Engine/EditorBlueprintResources/StandardMacros.IsValid` FromCell
    (:`Is Valid`
      (`/Engine/EditorBlueprintResources/StandardMacros.IsValid` ToCell
        (:`Is Valid`
          (`|ExecutionSequence`
            (:`then_0`
              (`NiagaraFunctionLibrary.SpawnSystemAtLocation` _returnvalue (`self.K2_GetActorLocation` FromCell)))
            (:`then_1`
              (`NiagaraFunctionLibrary.SpawnSystemAtLocation` _returnvalue (`self.K2_GetActorLocation`))))
          (`GameplayStatics.PlaySound2D` "/Game/SFX/Move.Move" 1.0 1.0 0.0 null null))))))

(event `UpdateShield`
  (`SceneComponent.SetVisibility` (`self.Shield`) (> (`self.GetHealth`) 1) false))

(event `OnSelect`
  (params (Attacking :type Boolean))
  (bind _billboard (`self.Billboard`))
  (`BillboardComponent.SetSprite` _billboard (select `bool` (`self.GetIsFriendly`) :`false` (select `bool` Attacking :`false` "/Game/Blueprints/UI/Textures/Icon_EnemyThinking.Icon_EnemyThinking" :`true` "/Game/Blueprints/UI/Textures/Icon_EnemyAttacking.Icon_EnemyAttacking" :!type "Texture2D Object Reference") :`true` "/Game/Blueprints/UI/Textures/Icon_PlayerHighlight.Icon_PlayerHighlight"))
  (`SceneComponent.SetVisibility` _billboard true false))

(event `OnDeselect`
  (`SceneComponent.SetVisibility` (`self.Billboard`) false false))

(event `self.HealthChanged`
  (`self.UpdateShield`))

(event `self.Death`
  (`self.K2_DestroyActor`))

(event `self.ReceiveAnyDamage`
  (params (Damage :type "Float (single-precision)") (DamageType :type "DamageType Object Reference") (InstigatedBy :type "Controller Object Reference") (DamageCauser :type "Actor Object Reference"))
  (`NiagaraFunctionLibrary.SpawnSystemAtLocation` "/Game/VFX/Flash/VFX_Impact.VFX_Impact" (+ (`self.K2_GetActorLocation`) (0.0 0.0 50.0))))

(fn `UserConstructionScript`)