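; Drag-and-drop operation for a card widget, handling both targeting cards and freely dragged cards.
; Targeting cards lazily create a viewport line from the drag origin to the pointer, while others follow the pointer through their canvas slot.
; During targeting, the player controller's cell under the cursor drives enter and leave notifications to the card.
; Drop notifies the card of the highlighted cell; drop and cancel both clear line and highlight, then end the drag.
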(event `self.Dragged`
  (params (PointerEvent :type "PointerEvent Structure (by ref)"))
  (bind _highlightedcell (`self.HighlightedCell`))
  (bind _card (`self.Card`))
  (bind _card_2 (`self.Card`))
  (`/Engine/EditorBlueprintResources/StandardMacros.IsValid` _card_2
    (:`Is Valid`
      (if (`/Game/Blueprints/Cards/CardBase.IsTargetingCard` _card_2)
        (`|ExecutionSequence`
          (:`then_0`
            ;[1 1 1] TargetingLine
            (`/Engine/EditorBlueprintResources/StandardMacros.IsValid` (`self.TargetingLine`)
              (:`Is Valid`
                (`/Game/Blueprints/UI/TargetingLine.UpdateTargetLocations` (`self.TargetingLine`) (`self.DragFrom`) (`KismetInputLibrary.PointerEvent_GetScreenSpacePosition` PointerEvent) :!label _label))
              (:`Is Not Valid`
                (`|ExecutionSequence`
                  (:`then_0`
                    (bind _line (`/Game/Blueprints/Cards/CardBase.CreateTargetingLine` (`self.Card`)))
                    (`UserWidget.AddToViewport` _line 0)
                    (set `self.TargetingLine` _line))
                  (:`then_1`
                    (goto _label))))))
          (:`then_1`
            ;[1 1 1] Notify card of cell highlighting
            (bind _asvoid_player_controller_bp (cast `/Game/Blueprints/VoidPlayerControllerBP` (`Widget.GetOwningPlayer` (`self.Card`))))
            (bind _cellundercursor (`/Game/Blueprints/VoidPlayerControllerBP.CellUnderCursor` _asvoid_player_controller_bp))
            (if (!= _cellundercursor (`self.HighlightedCell`))
              (`|ExecutionSequence`
                (:`then_0`
                  (`/Engine/EditorBlueprintResources/StandardMacros.IsValid` _highlightedcell
                    (:`Is Valid`
                      (`/Game/Blueprints/Cards/CardBase.CellDragLeave` (`self.Card`) _highlightedcell))))
                (:`then_1`
                  (bind _output_get (set `self.HighlightedCell` _cellundercursor))
                  (`/Engine/EditorBlueprintResources/StandardMacros.IsValid` _output_get
                    (:`Is Valid`
                      (`/Game/Blueprints/Cards/CardBase.CellDragEnter` (`self.Card`) _output_get))))))))
        (else
          ;[1 1 1] Drag card around
          (bind _returnvalue (`WidgetLayoutLibrary.GetPlayerScreenWidgetGeometry` (`Widget.GetOwningPlayer` _card)))
          (`CanvasPanelSlot.SetPosition` (`WidgetLayoutLibrary.SlotAsCanvasSlot` _card) (- (`SlateBlueprintLibrary.AbsoluteToLocal` _returnvalue (`KismetInputLibrary.PointerEvent_GetScreenSpacePosition` PointerEvent)) (`/Game/Blueprints/Cards/CardBase.DragOffset` _card))))))))

(event `self.Drop`
  (params (PointerEvent :type "PointerEvent Structure (by ref)"))
  (bind _highlightedcell (`self.HighlightedCell`))
  (bind _card (`self.Card`))
  (`KismetSystemLibrary.PrintString` null (`KismetTextLibrary.Conv_TextToString` (`|FormatText` "Dropped: {0} on {1}" (`self.CardName`) (`self.CellName`))))
  (`|ExecutionSequence`
    (:`then_0`
      (`/Engine/EditorBlueprintResources/StandardMacros.IsValid` _highlightedcell
        (:`Is Valid`
          (`/Game/Blueprints/Cards/CardBase.CellDragLeave` _card _highlightedcell)
          (`/Game/Blueprints/Cards/CardBase.CellDrop` _card _highlightedcell)
          (set `self.HighlightedCell` null))))
    (:`then_1`
      (`self.Cleanup`))))

(event `self.DragCancelled`
  (params (PointerEvent :type "PointerEvent Structure (by ref)"))
  (`KismetSystemLibrary.PrintString` null (`KismetTextLibrary.Conv_TextToString` (`|FormatText` "Drag canceled: {0}" (`self.CardName`))))
  (`self.Cleanup`))

(event `Cleanup`
  (bind _highlightedcell (`self.HighlightedCell`))
  (`|ExecutionSequence`
    (:`then_0`
      (`Widget.RemoveFromParent` (`self.TargetingLine`))
      (set `self.TargetingLine` null))
    (:`then_1`
      (`/Engine/EditorBlueprintResources/StandardMacros.IsValid` _highlightedcell
        (:`Is Valid`
          (`/Game/Blueprints/Cards/CardBase.CellDragLeave` (`self.Card`) _highlightedcell)
          (set `self.HighlightedCell` null))))
    (:`then_2`
      (`/Game/Blueprints/Cards/CardBase.DragEnd` (`self.Card`)))))