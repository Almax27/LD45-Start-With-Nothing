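; Game mode for a turn-based hex-map card game where the player wins if any friendly building survives the turn limit.
; EnterFlowState runs each phase of the parent's flow state machine: spawns, card draw and discard, enemy attacks, then enemy moves and telegraphs.
; Map and card completion events advance phases through DelayGotoNext, which reports an error if the state changed during its delay.
; Enemies resolve one by one through delayed, re-entrant event loops.
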(event `MapTransitionFinished`
  (params (HexMap :type "HexMap Object Reference"))
  ;[1 1 1] map load bindings
  (`self.DelayGotoNext` 0.5 "ShowBoard"))

(event `self.ReceiveBeginPlay`
  (`|ExecutionSequence`
    (:`then_0`
      ;[1 1 1] map load bindings
      (bind _returnvalue (`GameplayStatics.GetActorOfClass` "/Game/Blueprints/Map/HexMapBP.HexMapBP_C"))
      (bind _output_get (set `self.HexMapActor` _returnvalue))
      (add `HexMap.MapTransitionFinishedEvent` _output_get (delegate `MapTransitionFinished`)))
    (:`then_1`
      ;[1 1 1] Draw card binding
      (add `/Game/Blueprints/VoidPlayerControllerBP.CardDrawFinished` (`self.VoidPlayerController`) (delegate `CardDrawFinished`)))
    (:`then_2`
      ;[1 1 1] Discard cards binding
      (add `/Game/Blueprints/VoidPlayerControllerBP.CardDiscardFinished` (`self.VoidPlayerController`) (delegate `AllCardsDiscarded`)))
    (:`then_3`
      (`GameplayStatics.PlaySound2D` "/Game/SFX/MUSIC-pertho.MUSIC-pertho" 1.0 1.0 0.0 null self))))

(event `CardDrawFinished`
  ;[1 1 1] Draw card binding
  (`self.DelayGotoNext` 0.2 "PlayerDrawCards"))

(event `AllCardsDiscarded`
  ;[1 1 1] Discard cards binding
  (`self.DelayGotoNext` 0.5 "PlayerEndTurn"))

(event `self.EnterFlowState`
  (params (FlowState :type "EGameFlowStateType Enum" :default "None"))
  (bind _aitoresolve (`self.AIToResolve`))
  (bind _aitoresolve_2 (`self.AIToResolve`))
  (bind _returnvalue (`KismetArrayLibrary.Array_LastIndex` _aitoresolve))
  (bind _returnvalue_2 (`KismetArrayLibrary.Array_LastIndex` _aitoresolve_2))
  (`parent.EnterFlowState` FlowState)
  (switch `EGameFlowStateType` FlowState
    (:`GameStart`
      (set `self.TurnsRemaining` 5))
    (:`ShowBoard`
      (`self.SetMap` "/Game/Blueprints/Map/TileMap_1.TileMap_1"))
    (:`AddFirstPendingSpawns`
      (`self.AddFirstPendingSpawns`)
      (`GameplayStatics.PlaySound2D` "/Game/SFX/EnemyTurn.EnemyTurn" 1.0 1.0 0.0 null null)
      (`self.DelayGotoNext` 0.5 "AddFirstPendingSpawns"))
    (:`GameLoopStart`
      (`self.DelayGotoNext` 0.5 "GameLoopStart"))
    (:`SpawnEnemies`
      (`self.SpawnEnemies`)
      (`self.DelayGotoNext` 0.5 "SpawnEnemies"))
    (:`AddPendingSpawns`
      (`self.AddPendingSpawns`)
      (`self.DelayGotoNext` 0.5 "AddPendingSpawns"))
    (:`PlayerDrawCards`
      (`/Game/Blueprints/VoidPlayerControllerBP.DrawCards` (`self.VoidPlayerController`) 4))
    (:`PlayerPlayCards`
      (`GameplayStatics.PlaySound2D` "/Game/SFX/PlayersTurn.PlayersTurn" 1.0 1.0 0.0 null null))
    (:`PlayerEndTurn`
      (`/Game/Blueprints/VoidPlayerControllerBP.DiscardAllCards` (`self.VoidPlayerController`)))
    (:`ResolveEnemyAttacks`
      ;[1 1 1] Resolve ATtacks
      (`GameplayStatics.PlaySound2D` "/Game/SFX/EnemyTurn.EnemyTurn" 1.0 1.0 0.0 null null)
      (set `self.AIToResolve` (`self.GetEnemies`))
      (if (> (`KismetArrayLibrary.Array_Length` (`self.AIToResolve`)) 0) :!label _label
        (bind _asmap_entity_bp (cast `/Game/Blueprints/Map/Entities/MapEntityBP` (`|GetArrayItem` _aitoresolve_2 _returnvalue_2))
          (:`then`
            (if (`MapEntity.GetAIHasAttackPending` _asmap_entity_bp)
              (`/Game/Blueprints/Map/Entities/MapEntityBP.OnSelect` _asmap_entity_bp true)
              (`KismetSystemLibrary.Delay` 0.5)
              (`MapEntity.AIResolveAttack` _asmap_entity_bp)
              (`/Game/Blueprints/Map/Entities/MapEntityBP.OnDeselect` _asmap_entity_bp)))
          (:`CastFailed`
            _))
        (`KismetArrayLibrary.Array_Remove` _aitoresolve_2 _returnvalue_2)
        (`KismetSystemLibrary.Delay` 0.5)
        (bind _ended (`self.ResolveWinLoss`))
        (if (not _ended)
          (`self.ContinueToResolveAttacks`))
        (else
          (`self.DelayGotoNext` 0.5 "ResolveEnemyAttacks"))))
    (:`EnemyTurn`
      ;[1 1 1] Move/Telegraph
      (set `self.AIToResolve` (`self.GetEnemies`))
      (if (> (`KismetArrayLibrary.Array_Length` (`self.AIToResolve`)) 0) :!label _label_2
        (bind _asmap_entity_bp_2 (cast `/Game/Blueprints/Map/Entities/MapEntityBP` (`|GetArrayItem` _aitoresolve _returnvalue))
          (:`then`
            (`/Game/Blueprints/Map/Entities/MapEntityBP.OnSelect` _asmap_entity_bp_2 false)
            (`HexMap.HighlightCells` (`self.HexMapActor`) (`MapEntity.GetMoveLocations` _asmap_entity_bp_2) (`self.EnemyMoveColor`))
            (`KismetSystemLibrary.Delay` 0.5)
            (`MapEntity.AIMove` _asmap_entity_bp_2)
            (`KismetSystemLibrary.Delay` 0.5)
            (`HexMap.UnhighlightAllCells` (`self.HexMapActor`))
            (bind _returnvalue_3 (`MapEntity.AITelegraphAttack` _asmap_entity_bp_2))
            (if _returnvalue_3
              (`/Game/Blueprints/Map/Entities/MapEntityBP.OnSelect` _asmap_entity_bp_2 true)
              (else
                (`/Game/Blueprints/Map/Entities/MapEntityBP.OnDeselect` _asmap_entity_bp_2))))
          (:`CastFailed`
            _))
        (`KismetArrayLibrary.Array_Remove` _aitoresolve _returnvalue)
        (`KismetSystemLibrary.Delay` 0.5)
        (`self.ContinueToResolveMoves`)
        (else
          (`self.DelayGotoNext` 0.5 "EnemyTurn"))))
    (:`GameLoopEnd`
      (`/Engine/EditorBlueprintResources/StandardMacros.DecrementInt` (`self.TurnsRemaining`)
        (:`  `
          (`self.GotoNextFlowState`)
          (`self.ResolveWinLoss`))))
    (:`GameLost`
      (`self.SetMap` null :!label _label_3)
      (`KismetSystemLibrary.Delay` 5.0)
      (`self.GotoFlowState` "GameEnd"))
    (:`GameWon`
      (goto _label_3))
    (:`GameEnd`
      (bind _asvoid_player_controller_bp (cast `/Game/Blueprints/VoidPlayerControllerBP` (`GameplayStatics.GetPlayerController` 0)))
      (`GamePlayerController.ResetCards` _asvoid_player_controller_bp)
      (`self.GotoNextFlowState`))))

(event `ContinueToResolveAttacks`
  ;[1 1 1] Resolve ATtacks
  (goto _label))

(event `ContinueToResolveMoves`
  ;[1 1 1] Move/Telegraph
  (goto _label_2))

(fn `Goto`)

(fn `ResolveWinLoss`
  (returns (Ended :type Boolean))
  (locals (BuildingsRemaining :type Boolean))
  (`|ExecutionSequence`
    (:`then_0`
      (for _array_element (`self.GetFriendlies`)
        (cast `/Game/Blueprints/Map/Entities/Building` _array_element)
        (set `local.BuildingsRemaining` true)
        (break)))
    (:`then_1`
      (if (`local.BuildingsRemaining`)
        (if (== (`self.TurnsRemaining`) 0)
          (`self.GotoFlowState` "GameWon")
          (return true)
          (else
            (return false)))
        (else
          (`self.GotoFlowState` "GameLost")
          (return true))))))

(fn `SetMap`
  (params (Map :type "PaperTileMap Object Reference"))
  (`HexMap.SetTileMap` (`self.HexMapActor`) Map))

(fn `UserConstructionScript`)