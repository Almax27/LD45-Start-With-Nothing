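; Player controller for a hex-cell card game that owns the root HUD, advances the game mode out of GameStart and enables the HUD only during PlayerPlayCards.
; Tick line-traces under the cursor to track the hovered cell, and a click counts only when press and release hit the same cell.
; Delay loops draw and discard cards one by one, playing a shuffle when a draw fails.
; UseCard is an empty stub.
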(event `Key|F1`
  (params (Key :type "Key Structure"))
  (bind _helpswitcher (`/Game/Blueprints/UI/RootWidget.HelpSwitcher` (`self.RootWidget`)))
  (:`Pressed`
    (`WidgetSwitcher.SetActiveWidgetIndex` _helpswitcher (select `int` (`WidgetSwitcher.GetActiveWidgetIndex` _helpswitcher) :`0` 1 :`1` 0))))

(event `Key|AnyKey`
  (params (Key :type "Key Structure"))
  (:`Released`
    (bind _asvoid_game_mode_bp (cast `/Game/Blueprints/VoidGameModeBP` (`GameplayStatics.GetGameMode`)))
    (if (`|EnumEquality` (`VoidGameMode.GetCurrentFlowState` _asvoid_game_mode_bp) "GameStart")
      (`VoidGameMode.GotoNextFlowState` _asvoid_game_mode_bp))))

(event `self.ReceiveBeginPlay`
  (`|ExecutionSequence`
    (:`then_0`
      (bind _returnvalue (`|CreateWidget` "/Game/Blueprints/UI/RootWidget.RootWidget_C" self))
      (set `self.RootWidget` _returnvalue)
      (`UserWidget.AddToPlayerScreen` _returnvalue 0))
    (:`then_1`
      (bind _asvoid_game_mode_bp (cast `/Game/Blueprints/VoidGameModeBP` (`GameplayStatics.GetGameMode`)))
      (add `VoidGameMode.OnEnterFlowStateEvent` _asvoid_game_mode_bp (delegate `FlowStateChanged`)))))

(event `FlowStateChanged`
  (params (State :type "EGameFlowStateType Enum" :default "None"))
  (`self.SetRootWidgetEnabled` (`|EnumEquality` State "PlayerPlayCards")))

(event `self.ReceiveTick`
  (params (DeltaSeconds :type "Float (single-precision)"))
  (bind _returnvalue (`WidgetLayoutLibrary.GetMousePositionOnViewport`))
  (`self.UpdateCellUnderCusor` _returnvalue))

(event `DrawCards`
  (params (Max :type Integer))
  (bind _shuffling (`/Game/Blueprints/UI/RootWidget.Shuffling` (`self.RootWidget`)))
  (`KismetSystemLibrary.Delay` 0.15 :!label _label)
  (if (!= (`KismetArrayLibrary.Array_Length` (`self.HandCards`)) (`KismetMathLibrary.Min` Max (`KismetArrayLibrary.Array_Length` (`self.Deck`))))
    (bind _returnvalue (`self.DrawCard`))
    (`/Engine/EditorBlueprintResources/StandardMacros.IsValid` _returnvalue
      (:`Is Valid`
        (goto _label))
      (:`Is Not Valid`
        (`self.StartShuffle`)
        (`Widget.SetVisibility` _shuffling "HitTestInvisible")
        (`GameplayStatics.PlaySound2D` "/Game/SFX/CardShuffle.CardShuffle" 1.0 1.0 0.0 null null)
        (`KismetSystemLibrary.Delay` 1.0)
        (`Widget.SetVisibility` _shuffling "Hidden")
        (`self.EndShuffle`)
        (goto _label)))
    (else
      (`self.CardDrawFinished`))))

(event `DiscardAllCards`
  (bind _handcards (`self.HandCards`))
  (`KismetSystemLibrary.Delay` 0.15 :!label _label_2)
  (if (> (`KismetArrayLibrary.Array_Length` (`self.HandCards`)) 0)
    (`self.DiscardCard` (`|GetArrayItem` _handcards (`KismetArrayLibrary.Array_LastIndex` _handcards)))
    (goto _label_2)
    (else
      (`self.CardDiscardFinished`))))

(event `Key|LeftMouseButton`
  (params (Key :type "Key Structure"))
  (bind _cellundercursor (`self.CellUnderCursor`))
  (:`Pressed`
    (set `self.PressCell` _cellundercursor))
  (:`Released`
    (if (== _cellundercursor (`self.PressCell`))
      (`self.CellClicked` (`self.PressCell`))
      (set `self.PressCell` null))))

(event `UseCard`
  (params (Card :type "/Game/Blueprints/Cards/CardBase Object Reference"))
  (if (> (`CardWidget.Cost` Card) 0)
    _))

(event `Key|A`
  (params (Key :type "Key Structure")))

(fn `GetCellUnderCursor`
  (params (ScreenPosition :type "Vector2D Structure"))
  (returns (Cell :type "/Game/Blueprints/Map/Cells/BaseCell Object Reference"))
  (bind (_worldposition _worlddirection) (`GameplayStatics.DeprojectScreenToWorld` self (* ScreenPosition (`WidgetLayoutLibrary.GetViewportScale`))))
  (bind _outhit (`KismetSystemLibrary.LineTraceSingle` _worldposition (+ _worldposition (* _worlddirection 1000000.0)) "TraceTypeQuery1" true))
  (bind _asbase_cell (cast `/Game/Blueprints/Map/Cells/BaseCell` (`.HitActor` (`GameplayStatics.BreakHitResult` _outhit))))
  (return _asbase_cell))

(fn `SetRootWidgetEnabled`
  (params (Enabled :type Boolean))
  (`Widget.SetIsEnabled` (`/Game/Blueprints/UI/RootWidget.HUDRoot` (`self.RootWidget`)) Enabled))

(fn `UpdateCellUnderCusor`
  (params (ScreenPosition :type "Vector2D Structure"))
  (locals (NewCell :type "/Game/Blueprints/Map/Cells/BaseCell Object Reference"))
  (bind _output_get (set `local.NewCell` (`self.GetCellUnderCursor` ScreenPosition)))
  (if (!= _output_get (`self.CellUnderCursor`))
    (set `self.CellUnderCursor` (`local.NewCell`))))

(fn `UserConstructionScript`)